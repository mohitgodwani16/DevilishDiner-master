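; BP_DamageParent is a damage volume, named as a parent class, that hurts the player on entering it.
; Its construction script sizes the Collision box from a configurable extent.
; On begin overlap, an IsPlayer macro passes only player character 0, which then receives BaseDamage once per overlap, with a debug print of the amount.
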(event OnComponentBeginOverlap(Collision)
  (params (OverlappedComponent :type Primitive%20Component%20Object%20Reference) (OtherActor :type Actor%20Object%20Reference) (OtherComp :type Primitive%20Component%20Object%20Reference) (OtherBodyIndex :type Integer) (bFromSweep :type Boolean) (SweepResult :type Hit%20Result%20Structure%20%28by%20ref%29))
  (Utilities|IsPlayer? OtherActor
    (:IsPlayer
      (Game|Damage|ApplyDamage OtherActor (Variables|Default|GetBaseDamage) 0 self)
      (Development|PrintString (Utilities|String|Append "DamageDone: " (Utilities|String|ToString(Float) (Variables|Default|GetBaseDamage)))))))

(fn ConstructionScript
  (Components|Box|SetBoxExtent (Variables|Default|GetCollision) (Variables|Default|GetIn%20Box%20Extent) true))